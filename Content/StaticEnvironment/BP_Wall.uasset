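; BP_Wall is a modular mansion wall piece for static environment building.
; Its construction script sets the static mesh either to a random pick from the WallMeshes array or to one of four wall variants chosen by ChooseWallType, depending on UseRandomMesh.
; The event graph holds only disabled placeholder events, so it has no runtime logic.
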(fn `UserConstructionScript`
  (bind _staticmesh (`self.StaticMesh`))
  (if (`self.UseRandomMesh`)
    (`StaticMeshComponent.SetStaticMesh` (`self.StaticMesh`) (`KismetArrayLibrary.Array_Random` (`self.WallMeshes`)))
    (else
      (switch `int` (`self.ChooseWallType`)
        (:`0`
          (`StaticMeshComponent.SetStaticMesh` _staticmesh "/Game/StaticEnvironment/SM_Modular_Mansion_Set_SM_Wall1.SM_Modular_Mansion_Set_SM_Wall1"))
        (:`1`
          (`StaticMeshComponent.SetStaticMesh` _staticmesh "/Game/StaticEnvironment/SM_Modular_Mansion_Set_SM_Wall2.SM_Modular_Mansion_Set_SM_Wall2"))
        (:`2`
          (`StaticMeshComponent.SetStaticMesh` _staticmesh "/Game/StaticEnvironment/SM_Modular_Mansion_Set_SM_Wall3.SM_Modular_Mansion_Set_SM_Wall3"))
        (:`3`
          (`StaticMeshComponent.SetStaticMesh` _staticmesh "/Game/StaticEnvironment/SM_Modular_Mansion_Set_SM_Wall4.SM_Modular_Mansion_Set_SM_Wall4"))))))