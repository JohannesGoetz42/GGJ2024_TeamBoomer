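; Wall lamp Blueprint with a point light that can flicker at random.
; On BeginPlay, if Flickering is set, a one-shot timer starts the flicker event after LoopTime.
; The event sets a random light intensity, waits a random delay, then calls the flicker again, so LoopTime only delays the first flicker.
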(event `self.ReceiveBeginPlay`
  (if (`self.Flickering`)
    (`KismetSystemLibrary.K2_SetTimerDelegate` (delegate `E_Flicker`) (`self.LoopTime`))))

(event `E_Flicker`
  (`LightComponent.SetIntensity` (`self.PointLight`) (`KismetMathLibrary.RandomFloatInRange` 0.0 10000.0))
  (`KismetSystemLibrary.Delay` (`KismetMathLibrary.RandomFloatInRange` 0.0 2.0))
  (`self.E_Flicker`))

(fn `UserConstructionScript`)